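; BasePawn is a player-controlled camera pawn that orbits the world X axis, rolling to match its orbit angle.
; ScrollLeftRight changes the angle, ScrollUpDown slides the position along X as "zoom", and the mouse wheel steps the orbit radius as "altitude" within limits.
; UpdateCameraLocationRotation converts these values to a transform using sine and cosine, called from construction and the ScrollLeftRight axis event.
; PointOnASphere holds unused spherical math, and raising altitude prints a debug value.
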(event EventBeginPlay)

(event Collision|EventActorBeginOverlap
  (params (OtherActor :type Actor%20Object%20Reference)))

(event EventTick
  (params (DeltaSeconds :type Float%20%28single-precision%29)))

(event Input|ActionEvents|InputActionMouseWheelUp
  (params (Key :type Key%20Structure))
  (:Pressed
    (CallFunction|AdjustAltitude true)))

(event Input|ActionEvents|InputActionMouseWheelDown
  (params (Key :type Key%20Structure))
  (:Pressed
    (CallFunction|AdjustAltitude false)))

(event Input|AxisEvents|InputAxisScrollLeftRight
  (params (AxisValue :type Float%20%28single-precision%29))
  (Variables|Default|SetCamera%20X%20Rotation (+ (* AxisValue (Variables|Default|GetRotationSpeed)) (Variables|Default|GetCamera%20X%20Rotation)))
  (CallFunction|UpdateCameraLocation&Rotation))

(event Input|AxisEvents|InputAxisScrollUpDown
  (params (AxisValue :type Float%20%28single-precision%29))
  (CallFunction|AdjustZoom AxisValue))

(fn ConstructionScript
  (CallFunction|UpdateCameraLocation&Rotation))

(fn UpdateCameraLocation&Rotation
  (bind _camera_altitude (Variables|Default|GetCamera%20Altitude))
  (bind _camera_x_rotation (Variables|Default|GetCamera%20X%20Rotation))
  (Transformation|SetActorLocation (Math|Vector|MakeVector (Variables|Default|GetCamera%20Zoom) (* (Math|Trig|Sin(Degrees) _camera_x_rotation) _camera_altitude) (* (Math|Trig|Cos(Degrees) _camera_x_rotation) _camera_altitude)) false false)
  (Transformation|SetActorRotation (Math|Rotator|MakeRotator _camera_x_rotation 0.0 0.0)))

(fn AdjustAltitude
  (params (Increase :type Boolean))
  (if Increase
    (bind _output_get (Variables|Default|SetCamera%20Altitude (Math|Float|Min(Float) (+ (Variables|Default|GetCamera%20Altitude) (Variables|Default|GetAltitudeSpeed)) (Variables|Default|GetMax%20Altitude))))
    (Development|PrintText (Utilities|Text|ToText(Float) _output_get "HalfToEven"))
    (else
      (Variables|Default|SetCamera%20Altitude (Math|Float|Max(Float) (- (Variables|Default|GetCamera%20Altitude) (Variables|Default|GetAltitudeSpeed)) (Variables|Default|GetMin%20Altitude))))))

(fn AdjustZoom
  (params (Increase :type Float%20%28single-precision%29))
  (if (!= Increase 0.0)
    (if (>= Increase 1.0)
      (Variables|Default|SetCamera%20Zoom (Math|Float|Min(Float) (+ (Variables|Default|GetCamera%20Zoom) (* (Variables|Default|GetZoom%20Speed) Increase)) (Variables|Default|GetMin%20Zoom)))
      (else
        (Variables|Default|SetCamera%20Zoom (Math|Float|Max(Float) (Variables|Default|GetMax%20Zoom) (+ (Variables|Default|GetCamera%20Zoom) (* (Variables|Default|GetZoom%20Speed) Increase))))))))