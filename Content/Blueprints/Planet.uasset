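; Planet actor built at construction time from a Data value holding core size and layers.
; The construction script scales the core sphere by core size and adds one instanced mesh per layer, stepped diagonally in Y and Z.
; An unused CreateLayer function sketches procedural ring segments as YZ-plane quads via sine and cosine, but its angle math looks unfinished.
; The event graph has no active logic.
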(event EventBeginPlay)

(event Collision|EventActorBeginOverlap
  (params (OtherActor :type Actor%20Object%20Reference)))

(event EventTick
  (params (DeltaSeconds :type Float%20%28single-precision%29)))

(fn ConstructionScript
  (bind _data (Variables|Default|GetData))
  (bind (_name _layers _coresize) (Utilities|Struct|BreakPlanetStruct _data))
  (Transformation|SetWorldScale3D (Variables|Default|GetSphere) (* "1.000000,1.000000,1.000000" _coresize))
  (for (_array_element _array_index) _layers
    (Components|InstancedStaticMesh|AddInstance (Variables|Default|GetInstancedStaticMesh) (Math|Transform|MakeTransform (Math|Vector|MakeVector 0.0 (* _array_index 5.0) (* _array_index 5.0))))))

(fn CreateLayer
  (params (Layer :type Layer%20Struct%20Structure) (LayerHeightOffset :type Float%20%28single-precision%29))
  (bind (_height _segmentcount) (Utilities|Struct|BreakLayerStruct Layer))
  (bind _output_get (LocalVariables|SetSegmentOffsetHeight LayerHeightOffset))
  (bind _output_get_2 (LocalVariables|SetSegmentOffsetAngle 3e+01))
  (bind _output_get_3 (LocalVariables|SetSegmentCoreAngle (/ 3.6e+02 _segmentcount)))
  (for _index (range 0 (Math|Float|Truncate _segmentcount))
    (Class|ProceduralMeshComponent|CreateMeshSectionLinearColor (Variables|Default|GetProceduralMesh) _index (Utilities|Array|MakeArray (Math|Vector|MakeVector 0.0 (Math|Trig|Sin(Degrees) (* _index _output_get_3)) (Math|Trig|Cos(Degrees) (* _index _output_get_3))) (Math|Vector|MakeVector 0.0 (Math|Trig|Sin(Degrees) (* (+ _index 1) _output_get_3)) (Math|Trig|Cos(Degrees) (* (+ _index 1) _output_get_3))) (Math|Vector|MakeVector 0.0 (* (+ _output_get _height) (Math|Trig|Sin(Degrees) (* _index 0.0))) (* (+ _output_get _height) (Math|Trig|Cos(Degrees) (* _index 0.0)))) (Math|Vector|MakeVector 0.0 (* (+ _output_get _height) (Math|Trig|Sin(Degrees) (* (+ _index 1) 0.0))) (* (+ _output_get _height) (Math|Trig|Cos(Degrees) (* (+ _index 1) 0.0))))) (Utilities|Array|MakeArray 0 1 2 3 2 1) (Utilities|Array|MakeArray "0, 0, 0") 0 0 0 false)
    (LocalVariables|SetSegmentCoreAngle (+ _output_get_2 _output_get_3))))