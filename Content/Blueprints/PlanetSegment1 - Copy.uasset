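; Procedural mesh actor that builds a curved segment of a planet, judging by its name, in the construction script.
; CalculateVerticies uses sine and cosine to fill front and back, top and bottom arc points from width, height, offset, angle and subdivisions.
; Only the front face is meshed, with collision, from interleaved top and bottom points.
; Triangle indices use a hardcoded range and, like the mesh section, are regenerated on every vertex-loop pass, alongside a debug print.
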(event EventBeginPlay)

(event Collision|EventActorBeginOverlap
  (params (OtherActor :type Actor%20Object%20Reference)))

(event EventTick
  (params (DeltaSeconds :type Float%20%28single-precision%29)))

(fn ConstructionScript
  (bind _verticies (LocalVariables|GetVerticies))
  (bind _triangles (LocalVariables|GetTriangles))
  (CallFunction|CalculateVerticies)
  (for (_array_element _array_index) (Variables|Default|GetFrontTop)
    (bind _returnvalue (Utilities|Array|Add _verticies _array_element))
    (Utilities|Array|Add _verticies (Utilities|Array|Get(acopy) (Variables|Default|GetFrontBottom) _array_index))
    (Development|PrintText (Utilities|Text|ToText(Integer) _returnvalue))
    (for _index (range -1 32)
      (Utilities|Array|Add _triangles _index)
      (Utilities|Array|Add _triangles (+ _index 1))
      (Utilities|Array|Add _triangles (+ (+ _index 1) 1))
      (Utilities|Array|Add _triangles (+ (+ _index 1) 1))
      (Utilities|Array|Add _triangles (+ _index 1))
      (Utilities|Array|Add _triangles (+ (+ (+ _index 1) 1) 1)))
    (Class|ProceduralMeshComponent|CreateMeshSectionLinearColor (Variables|Default|GetFront) 0 _verticies _triangles 0 0 0 0 true)))

(fn CalculateVerticies
  (bind _heightoffset (Variables|Default|GetHeightOffset))
  (bind _heightoffset_2 (Variables|Default|GetHeightOffset))
  (bind _height (Variables|Default|GetHeight))
  (bind _width (Variables|Default|GetWidth))
  (bind _subsegments (Variables|Default|GetSubSegments))
  (bind _angle (Variables|Default|GetAngle))
  (bind _heightoffset_3 (Variables|Default|GetHeightOffset))
  (bind _heightoffset_4 (Variables|Default|GetHeightOffset))
  (bind _height_2 (Variables|Default|GetHeight))
  (bind _width_2 (Variables|Default|GetWidth))
  (bind _returnvalue (/ _width 2.0))
  (bind _returnvalue_2 (/ _width_2 2.0))
  (bind _returnvalue_3 (Math|Conversions|ToFloat(Integer) _subsegments))
  (bind _returnvalue_4 (+ _heightoffset_3 _height_2))
  (bind _returnvalue_5 (+ _heightoffset _height))
  (bind _returnvalue_6 (/ _angle _returnvalue_3))
  (bind _returnvalue_7 (* _returnvalue -1.0))
  (bind _returnvalue_8 (* _returnvalue_2 -1.0))
  (Utilities|Array|Insert (Variables|Default|GetFrontBottom) (Math|Vector|MakeVector _returnvalue_2 0.0 _heightoffset_4))
  (Utilities|Array|Insert (Variables|Default|GetFrontTop) (Math|Vector|MakeVector _returnvalue_2 0.0 _returnvalue_4))
  (Utilities|Array|Insert (Variables|Default|GetBackBottom) (Math|Vector|MakeVector _returnvalue_8 0.0 _heightoffset_4))
  (Utilities|Array|Insert (Variables|Default|GetBackTop) (Math|Vector|MakeVector _returnvalue_8 0.0 _returnvalue_4))
  (for _index (range 1 _subsegments)
    (Utilities|Array|Insert (Variables|Default|GetFrontBottom) (Math|Vector|MakeVector _returnvalue (* (Math|Trig|Sin(Degrees) (* _index _returnvalue_6)) _heightoffset_2) (* (Math|Trig|Cos(Degrees) (* _index _returnvalue_6)) _heightoffset_2)))
    (Utilities|Array|Insert (Variables|Default|GetFrontTop) (Math|Vector|MakeVector _returnvalue (* (Math|Trig|Sin(Degrees) (* _index _returnvalue_6)) _returnvalue_5) (* (Math|Trig|Cos(Degrees) (* _index _returnvalue_6)) _returnvalue_5)))
    (Utilities|Array|Insert (Variables|Default|GetBackBottom) (Math|Vector|MakeVector _returnvalue_7 (* (Math|Trig|Sin(Degrees) (* (+ _index 1) _returnvalue_6)) _heightoffset_2) (* (Math|Trig|Cos(Degrees) (* (+ _index 1) _returnvalue_6)) _heightoffset_2)))
    (Utilities|Array|Insert (Variables|Default|GetBackTop) (Math|Vector|MakeVector _returnvalue_7 (* (Math|Trig|Sin(Degrees) (* (+ _index 1) _returnvalue_6)) _returnvalue_5) (* (Math|Trig|Cos(Degrees) (* (+ _index 1) _returnvalue_6)) _returnvalue_5)))))